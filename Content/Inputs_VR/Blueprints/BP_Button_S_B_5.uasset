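; VR cockpit push button that sinks slightly when the ZeroGPlayer overlaps its sphere and returns when the overlap ends.
; On BeginPlay it finds the BP_Ship and teleports its mesh to a Cockpit socket whose name is derived from the component name minus BlenderName, using configured rotation values.
; Tick re-attaches to the hardcoded S_B_1 socket every frame, keeping world transform.
; The press is purely positional, triggering no other action.
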(event OnComponentBeginOverlap(Sphere)
  (params (OverlappedComponent :type Primitive%20Component%20Object%20Reference) (OtherActor :type Actor%20Object%20Reference) (OtherComp :type Primitive%20Component%20Object%20Reference) (OtherBodyIndex :type Integer) (bFromSweep :type Boolean) (SweepResult :type Hit%20Result%20Structure%20%28by%20ref%29))
  (Utilities|Casting|CastToZeroGPlayer OtherActor)
  (Components|MoveComponentTo (Variables|Default|GetButton) (- (Variables|Default|GetButtonStart) "0.000000,0.000000,0.500000") "0, 0, 0" false false 0.1 false))

(event OnComponentEndOverlap(Sphere)
  (params (OverlappedComponent :type Primitive%20Component%20Object%20Reference) (OtherActor :type Actor%20Object%20Reference) (OtherComp :type Primitive%20Component%20Object%20Reference) (OtherBodyIndex :type Integer))
  (Utilities|Casting|CastToZeroGPlayer OtherActor)
  (Components|MoveComponentTo (Variables|Default|GetButton) (Variables|Default|GetButtonStart) "0, 0, 0" false false 0.1 false))

(event EventBeginPlay
  (bind _flick__5__s_b_1 (Variables|Default|GetFlick__5__S_B_1))
  (Utilities|FlowControl|Sequence
    (:then_0
      (Variables|Default|SetButtonStart (Variables|/Script/Engine.SceneComponent|GetRelativeLocation (Variables|Default|GetButton))))
    (:then_1
      (bind _returnvalue (Actor|GetActorOfClass "/Game/Zero_Gravity/Blueprints/ZeroGPlayer.ZeroGPlayer_C"))
      (Variables|Default|SetActor _returnvalue)
      (bind _returnvalue_2 (Actor|GetActorOfClass "/Game/SpaceShip/BP_Ship.BP_Ship_C"))
      (Variables|Default|SetBP_Ship _returnvalue_2)
      (Transformation|SetWorldTransform _flick__5__s_b_1 (Math|Transform|MakeTransform (Transformation|GetSocketLocation (Variables|/Game/SpaceShip/BP_Ship.BP_Ship_C|GetCockpit (Variables|Default|GetBP_Ship)) (Utilities|String|StringToName (Utilities|String|Replace (Utilities|GetObjectName _flick__5__s_b_1) (Utilities|String|ToString(Text) (Variables|Default|GetBlender_Name))))) (Math|Rotator|MakeRotator (Variables|Default|GetX%20%28Roll%29) (Variables|Default|GetY%20%28Pitch%29) (Variables|Default|GetZ%20%28Yaw%29)) "1.000000,1.000000,1.000000") false true))))

(event EventTick
  (params (DeltaSeconds :type Float%20%28single-precision%29))
  (Utilities|FlowControl|Sequence
    (:then_0
      (if (Utilities|Operators|EqualEqual :A (Variables|/Script/Engine.SceneComponent|GetRelativeLocation (Variables|Default|GetButton)))
        _))
    (:then_1
      (Transformation|AttachComponentToComponent (Variables|/Game/SpaceShip/BP_Ship.BP_Ship_C|GetCockpit (Variables|Default|GetBP_Ship)) "S_B_1" "KeepWorld" "KeepWorld" "KeepWorld" true))))

(fn ConstructionScript)
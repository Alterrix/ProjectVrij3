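; VR cockpit joystick that finds the ship on BeginPlay and mounts to its cockpit socket, re-attaching every Tick.
; While grabbed, a looping timer pins the player's right hand to the grip and tilts the stick toward the motion controller using look-at dot products, with clamped pitch and roll.
; Tick converts the tilt into centred X/Y axis variables; nothing here applies them to the ship.
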(event FirstHandGrabbed(C_GrabComponent)
  (params (Motion%20Controller :type Motion%20Controller%20Component%20Object%20Reference) (SkeltalMeshHand :type Skeletal%20Mesh%20Component%20Object%20Reference) (Motion%20Controller%20Aim :type Motion%20Controller%20Component%20Object%20Reference))
  ;[1 1 1] Calculate left Right Position
  (Variables|Default|SetMotion%20Controller Motion%20Controller))

(event FirstHandDropped(C_GrabComponent)
  (params (Original%20Hand%20Location :type Transform) (Motion%20Controller :type Motion%20Controller%20Component%20Object%20Reference) (Skeletal%20Mesh%20Hand :type Skeletal%20Mesh%20Component%20Object%20Reference))
  (Class|KismetSystemLibrary|PauseTimer 0 "Update Position")
  ;[1 1 1] Calculate left Right Position
  (Variables|Default|SetMotion%20Controller 0))

(event Custom|Update%20Position
  (bind _joystick (Variables|Default|GetJoyStick))
  (bind _motion_controller (Variables|Default|GetMotion%20Controller))
  (bind _joystick_2 (Variables|Default|GetJoyStick))
  (bind _motion_controller_2 (Variables|Default|GetMotion%20Controller))
  (bind _joystick_3 (Variables|Default|GetJoyStick))
  (bind _joystick_4 (Variables|Default|GetJoyStick))
  (bind _joystick_5 (Variables|Default|GetJoyStick))
  (bind _returnvalue (Transformation|GetWorldRotation _joystick))
  (bind _returnvalue_2 (Transformation|GetWorldLocation _joystick))
  (bind _returnvalue_3 (Transformation|GetWorldLocation _motion_controller))
  (bind _returnvalue_4 (Transformation|GetWorldRotation _joystick_3))
  (bind _returnvalue_5 (Transformation|GetWorldLocation _joystick_3))
  (bind _returnvalue_6 (Transformation|GetWorldLocation _motion_controller_2))
  (bind _relativerotation (Variables|/Script/Engine.SceneComponent|GetRelativeRotation _joystick_4))
  (bind _relativerotation_2 (Variables|/Script/Engine.SceneComponent|GetRelativeRotation _joystick_4))
  (bind _relativerotation_3 (Variables|/Script/Engine.SceneComponent|GetRelativeRotation _joystick_5))
  (bind _relativerotation_4 (Variables|/Script/Engine.SceneComponent|GetRelativeRotation _joystick_2))
  (bind _returnvalue_7 (Math|Rotator|FindLookatRotation _returnvalue_5 _returnvalue_6))
  (bind _returnvalue_8 (Math|Vector|GetForwardVector _returnvalue_4))
  (bind _returnvalue_9 (Math|Vector|GetRightVector _returnvalue))
  (bind _returnvalue_10 (Math|Rotator|FindLookatRotation _returnvalue_2 _returnvalue_3))
  (bind _returnvalue_11 (Math|Rotator|GetRotationXVector _returnvalue_10))
  (bind _returnvalue_12 (Math|Rotator|GetRotationXVector _returnvalue_7))
  (bind _returnvalue_13 (* _returnvalue_8 -1.0))
  (bind _returnvalue_14 (Math|Vector|DotProduct _returnvalue_11 _returnvalue_9))
  (bind _returnvalue_15 (Math|Vector|DotProduct _returnvalue_12 _returnvalue_13))
  (bind _returnvalue_16 (* _returnvalue_15 1e+01))
  (bind _returnvalue_17 (* _returnvalue_14 1e+01))
  (bind _returnvalue_18 (Math|Rotator|MakeRotator _returnvalue_17 _returnvalue_16 0.0))
  ;[1 1 1] Calculate left Right Position
  (Transformation|SetWorldLocation (Variables|/Game/Zero_Gravity/Blueprints/ZeroGPlayer.ZeroGPlayer_C|GetHandRight (Variables|Default|GetPlayer)) (Transformation|GetWorldLocation (Variables|Default|GetgrabPoint)) false false)
  (Transformation|AddRelativeRotation _joystick_4 (Math|Rotator|MakeRotator (.roll _returnvalue_18) (.pitch _returnvalue_18) 0.0) false false)
  (Utilities|FlowControl|Sequence
    (:then_0
      (if (>= (.roll _relativerotation_2) 3e+01)
        (Development|PrintString "Hello")
        (Transformation|SetRelativeRotation _joystick_5 (Math|Rotator|MakeRotator 3e+01 (.pitch _relativerotation_3) 0.0) false false)))
    (:then_1
      (if (>= (.pitch _relativerotation_2) 3e+01)
        (Transformation|SetRelativeRotation _joystick_5 (Math|Rotator|MakeRotator (.roll _relativerotation_3) 3e+01 0.0) false false)))
    (:then_2
      (if (<= (.roll _relativerotation) -3e+01)
        (Transformation|SetRelativeRotation _joystick_2 (Math|Rotator|MakeRotator -3e+01 (.pitch _relativerotation_4) 0.0) false false)))
    (:then_3
      (if (<= (.pitch _relativerotation) -3e+01)
        (Transformation|SetRelativeRotation _joystick_2 (Math|Rotator|MakeRotator (.roll _relativerotation_4) -3e+01 0.0) false false)))))

(event EventBeginPlay
  (bind _returnvalue (Actor|GetActorOfClass "/Game/SpaceShip/BP_Ship.BP_Ship_C"))
  (Variables|Default|SetBP_Ship _returnvalue)
  (Transformation|SetWorldTransform (Variables|Default|GetC_J_1) (Math|Transform|MakeTransform (Transformation|GetSocketLocation (Variables|/Game/SpaceShip/BP_Ship.BP_Ship_C|GetCockpit (Variables|Default|GetBP_Ship)) (Utilities|String|StringToName (Utilities|String|Replace (Utilities|GetObjectName (Variables|Default|GetC_J_1)) (Utilities|String|ToString(Text) (Variables|Default|GetBlender_Name))))) (Math|Rotator|MakeRotator (Variables|Default|GetX%20%28Roll%29) (Variables|Default|GetY%20%28Pitch%29) (Variables|Default|GetZ%20%28Yaw%29)) "1.000000,1.000000,1.000000") false true)
  (bind _returnvalue_2 (Actor|GetActorOfClass "/Game/Zero_Gravity/Blueprints/ZeroGPlayer.ZeroGPlayer_C"))
  (Variables|Default|SetPlayer _returnvalue_2))

(event EventTick
  (params (DeltaSeconds :type Float%20%28single-precision%29))
  (bind _joystick (Variables|Default|GetJoyStick))
  (bind _relativerotation (Variables|/Script/Engine.SceneComponent|GetRelativeRotation _joystick))
  ;[1 1 1] Calculate left Right Position
  (Utilities|FlowControl|Sequence
    (:then_0
      (bind _output_get (Variables|Default|SetVariable%20max%20y (- (Math|Float|MapRangeClamped (* (/ (+ (.roll _relativerotation) 3e+01) 6e+01) 1e+02) 0.0 1e+02 0.0 1.0) 0.5))))
    (:then_1
      (bind _output_get_2 (Variables|Default|Setvariable%20max%20x (- (Math|Float|MapRangeClamped (* (/ (+ (.pitch _relativerotation) 3e+01) 6e+01) 1e+02) 0.0 1e+02 0.0 1.0) 0.5))))
    (:then_2
      (Transformation|AttachComponentToComponent (Variables|/Game/SpaceShip/BP_Ship.BP_Ship_C|GetCockpit (Variables|Default|GetBP_Ship)) "C_J_1" "SnapToTarget" "KeepWorld" "KeepWorld" true))))

(event EventGrab
  (params (MotionController :type Motion%20Controller%20Component%20Object%20Reference))
  ;[1 1 1] Calculate left Right Position
  (Variables|Default|SetMotion%20Controller MotionController)
  (Utilities|Time|SetTimerbyEvent (delegate Custom|Update%20Position) 0.01 true))

(event EventRelease
  (params (MotionController :type Motion%20Controller%20Component%20Object%20Reference))
  ;[1 1 1] Calculate left Right Position
  (if (== MotionController (Variables|Default|GetMotion%20Controller))
    (Class|KismetSystemLibrary|PauseTimer 0 "Update Position")
    (Variables|Default|SetMotion%20Controller 0)))

(fn ConstructionScript)
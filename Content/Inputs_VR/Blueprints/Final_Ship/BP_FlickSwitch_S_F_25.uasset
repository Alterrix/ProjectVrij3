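; VR cockpit flick switch that snaps its visual between two rotations and flips an OnOff flag when the player pawn overlaps it.
; On BeginPlay it finds BP_Ship and moves itself to a Cockpit socket whose name comes from its object name via string replace.
; Tick re-runs a keep-world attach to the hard-coded S_F_10 socket every frame.
; A DoOnce reset after a short delay debounces toggling, which drives no other ship system here.
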(event OnComponentBeginOverlap(SwitchFlick)
  (params (OverlappedComponent :type Primitive%20Component%20Object%20Reference) (OtherActor :type Actor%20Object%20Reference) (OtherComp :type Primitive%20Component%20Object%20Reference) (OtherBodyIndex :type Integer) (bFromSweep :type Boolean) (SweepResult :type Hit%20Result%20Structure%20%28by%20ref%29))
  (bind _switch (Variables|Default|GetSwitch))
  (if (== (Game|Player|GetPlayerPawn 0) OtherActor)
    (Utilities|FlowControl|DoOnce false :!label _label
      (:Completed
        (if (Variables|Default|GetOn/Off)
          (Transformation|SetRelativeRotation _switch (Math|Rotator|MakeRotator -4e+01 0.0 -2.7e+02) false false)
          (Variables|Default|SetOn/Off false)
          (else
            (Transformation|SetRelativeRotation _switch (Math|Rotator|MakeRotator -1.2e+02 0.0 -2.7e+02) false false)
            (Variables|Default|SetOn/Off true)))
        (Utilities|FlowControl|Delay 1.0)
        (goto _label Reset)))))

(event EventBeginPlay
  (bind _flick__5__s_f_10 (Variables|Default|GetFlick__5__S_F_10))
  (bind _returnvalue (Actor|GetActorOfClass "/Game/Zero_Gravity/Blueprints/ZeroGPlayer.ZeroGPlayer_C"))
  (Variables|Default|SetActor _returnvalue)
  (bind _returnvalue_2 (Actor|GetActorOfClass "/Game/SpaceShip/BP_Ship.BP_Ship_C"))
  (Variables|Default|SetBP_Ship _returnvalue_2)
  (Transformation|SetWorldTransform _flick__5__s_f_10 (Math|Transform|MakeTransform (Transformation|GetSocketLocation (Variables|/Game/SpaceShip/BP_Ship.BP_Ship_C|GetCockpit (Variables|Default|GetBP_Ship)) (Utilities|String|StringToName (Utilities|String|Replace (Utilities|GetObjectName _flick__5__s_f_10) (Utilities|String|ToString(Text) (Variables|Default|GetBlender_Name))))) (Math|Rotator|MakeRotator (Variables|Default|GetX%20%28Roll%29) (Variables|Default|GetY%20%28Pitch%29) (Variables|Default|GetZ%20%28Yaw%29)) "1.000000,1.000000,1.000000") false true))

(event EventTick
  (params (DeltaSeconds :type Float%20%28single-precision%29))
  (Transformation|AttachComponentToComponent (Variables|/Game/SpaceShip/BP_Ship.BP_Ship_C|GetCockpit (Variables|Default|GetBP_Ship)) "S_F_10" "KeepWorld" "KeepWorld" "KeepWorld" true))

(fn ConstructionScript)
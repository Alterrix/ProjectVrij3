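; VR cockpit flick switch actor that sits at the Bone_Button_chair_J_FORW socket on the spaceship's cockpit.
; On BeginPlay it finds the player, ship and joystick, then moves its component to a socket whose name is derived from the component's own name.
; Tick re-runs the attachment to that cockpit socket every frame.
; Sphere overlap by ZeroGPlayer only prints a debug "hit"; no switch action is wired.
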(event OnComponentBeginOverlap(Sphere)
  (params (OverlappedComponent :type Primitive%20Component%20Object%20Reference) (OtherActor :type Actor%20Object%20Reference) (OtherComp :type Primitive%20Component%20Object%20Reference) (OtherBodyIndex :type Integer) (bFromSweep :type Boolean) (SweepResult :type Hit%20Result%20Structure%20%28by%20ref%29))
  (Utilities|Casting|CastToZeroGPlayer OtherActor)
  (Development|PrintString "hit"))

(event EventBeginPlay
  (bind _flick__5__bone_button_chair_j_forw (Variables|Default|GetFlick__5__Bone_Button_chair_J_FORW))
  (Utilities|FlowControl|Sequence
    (:then_1
      (bind _returnvalue (Actor|GetActorOfClass "/Game/Zero_Gravity/Blueprints/ZeroGPlayer.ZeroGPlayer_C"))
      (Variables|Default|SetActor _returnvalue)
      (bind _returnvalue_2 (Actor|GetActorOfClass "/Game/SpaceShip/SpaceShip_Final1.SpaceShip_Final1_C"))
      (Variables|Default|SetBP_Ship _returnvalue_2)
      (bind _returnvalue_3 (Actor|GetActorOfClass "/Game/Inputs_VR/Blueprints/Final_Ship/Real_Final/JoyStick_Spaceship_final1.JoyStick_Spaceship_final1_C"))
      (Variables|Default|Setjoystick%20spaceship _returnvalue_3)
      (Transformation|SetWorldTransform _flick__5__bone_button_chair_j_forw (Math|Transform|MakeTransform (Transformation|GetSocketLocation (Variables|/Game/SpaceShip/SpaceShip_Final1.SpaceShip_Final1_C|GetCockpit (Variables|Default|GetBP_Ship)) (Utilities|String|StringToName (Utilities|String|Replace (Utilities|GetObjectName _flick__5__bone_button_chair_j_forw) (Utilities|String|ToString(Text) (Variables|Default|GetBlender_Name))))) (Math|Rotator|MakeRotator (Variables|Default|GetX%20%28Roll%29) (Variables|Default|GetY%20%28Pitch%29) 0.0) "1.000000,1.000000,1.000000") false true))))

(event EventTick
  (params (DeltaSeconds :type Float%20%28single-precision%29))
  (Utilities|FlowControl|Sequence
    (:then_1
      (Transformation|AttachComponentToComponent (Variables|/Game/SpaceShip/SpaceShip_Final1.SpaceShip_Final1_C|GetCockpit (Variables|Default|GetBP_Ship)) "Bone_Button_chair_J_FORW" "KeepWorld" "KeepRelative" "KeepWorld" true))))

(fn ConstructionScript)
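; VR cockpit flick switch that turns the blinking wing lights on SpaceShip_Final1 on and off.
; BeginPlay places it at a cockpit socket derived from its object name, and Tick re-attaches it to Bone_Switch_WNGLT every frame.
; Player pawn overlap flips the switch unless the thruster is grabbed, with a DoOnce and delay as debounce.
; A looping timer blinks one light pair and chains a delayed timer for the second, or hides all when off.
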(event OnComponentBeginOverlap(SwitchFlick)
  (params (OverlappedComponent :type Primitive%20Component%20Object%20Reference) (OtherActor :type Actor%20Object%20Reference) (OtherComp :type Primitive%20Component%20Object%20Reference) (OtherBodyIndex :type Integer) (bFromSweep :type Boolean) (SweepResult :type Hit%20Result%20Structure%20%28by%20ref%29))
  (bind _switch (Variables|Default|GetSwitch))
  (if (== (Game|Player|GetPlayerPawn 0) OtherActor)
    (Utilities|FlowControl|DoOnce false :!label _label
      (:Completed
        (if (not (Variables|/Game/Inputs_VR/Blueprints/Final_Ship/Real_Final/Thruster_SpaceShip_final1.Thruster_SpaceShip_final1_C|GetGrabbed (Variables|Default|GetThrusterSpaceShip)))
          (if (Variables|Default|GetOn/Off)
            (Transformation|SetRelativeRotation _switch (Math|Rotator|MakeRotator -4e+01 0.0 -2.7e+02) false false)
            (Variables|Default|SetOn/Off false)
            (else
              (Transformation|SetRelativeRotation _switch (Math|Rotator|MakeRotator -1.2e+02 0.0 -2.7e+02) false false)
              (Variables|Default|SetOn/Off true)))
          (Utilities|Time|SetTimerbyFunctionName 0 "TimerLightWNGL" 1.0 true)
          (Utilities|FlowControl|Delay 1.0)
          (goto _label Reset))))))

(event EventBeginPlay
  (bind _flick__5__bone_switch_wnglt (Variables|Default|GetFlick__5__Bone_Switch_WNGLT))
  (bind _returnvalue (Actor|GetActorOfClass "/Game/Zero_Gravity/Blueprints/ZeroGPlayer.ZeroGPlayer_C"))
  (Variables|Default|SetActor _returnvalue)
  (bind _returnvalue_2 (Actor|GetActorOfClass "/Game/SpaceShip/SpaceShip_Final1.SpaceShip_Final1_C"))
  (Variables|Default|SetBP_Ship _returnvalue_2)
  (bind _returnvalue_3 (Actor|GetActorOfClass "/Game/Inputs_VR/Blueprints/Final_Ship/Real_Final/Thruster_SpaceShip_final1.Thruster_SpaceShip_final1_C"))
  (Variables|Default|SetThrusterSpaceShip _returnvalue_3)
  (Transformation|SetWorldTransform _flick__5__bone_switch_wnglt (Math|Transform|MakeTransform (Transformation|GetSocketLocation (Variables|/Game/SpaceShip/SpaceShip_Final1.SpaceShip_Final1_C|GetCockpit (Variables|Default|GetBP_Ship)) (Utilities|String|StringToName (Utilities|String|Replace (Utilities|GetObjectName _flick__5__bone_switch_wnglt) (Utilities|String|ToString(Text) (Variables|Default|GetBlender_Name))))) (Math|Rotator|MakeRotator (Variables|Default|GetX%20%28Roll%29) (Variables|Default|GetY%20%28Pitch%29) (Variables|Default|GetZ%20%28Yaw%29)) "1.000000,1.000000,1.000000") false true))

(event EventTick
  (params (DeltaSeconds :type Float%20%28single-precision%29))
  (Transformation|AttachComponentToComponent (Variables|/Game/SpaceShip/SpaceShip_Final1.SpaceShip_Final1_C|GetCockpit (Variables|Default|GetBP_Ship)) "Bone_Switch_WNGLT" "KeepWorld" "KeepWorld" "KeepWorld" true))

(fn ConstructionScript)

(fn TimerLightWNGR
  (bind _bp_ship (Variables|Default|GetBP_Ship))
  (bind _bp_ship_2 (Variables|Default|GetBP_Ship))
  (if (Variables|Default|GetOn/Off)
    (if (Variables|Default|GetLTB2)
      (Development|SetHiddeninGame (Variables|/Game/SpaceShip/SpaceShip_Final1.SpaceShip_Final1_C|GetWNGLT2 _bp_ship_2) true false)
      (Development|SetHiddeninGame (Variables|/Game/SpaceShip/SpaceShip_Final1.SpaceShip_Final1_C|GetWNGLT4 _bp_ship_2) true false)
      (Variables|Default|SetLTB2 false)
      (else
        (Development|SetHiddeninGame (Variables|/Game/SpaceShip/SpaceShip_Final1.SpaceShip_Final1_C|GetWNGLT2 _bp_ship) false false :!label _label)
        (Development|SetHiddeninGame (Variables|/Game/SpaceShip/SpaceShip_Final1.SpaceShip_Final1_C|GetWNGLT4 _bp_ship) false false)
        (Variables|Default|SetLTB2 true)))
    (else
      (goto _label))))

(fn TimerLightWNGL
  (bind _bp_ship (Variables|Default|GetBP_Ship))
  (bind _bp_ship_2 (Variables|Default|GetBP_Ship))
  (bind _bp_ship_3 (Variables|Default|GetBP_Ship))
  (if (Variables|Default|GetOn/Off)
    (if (Variables|Default|GetLTB1)
      (Development|SetHiddeninGame (Variables|/Game/SpaceShip/SpaceShip_Final1.SpaceShip_Final1_C|GetWNGLT _bp_ship_2) true false)
      (Development|SetHiddeninGame (Variables|/Game/SpaceShip/SpaceShip_Final1.SpaceShip_Final1_C|GetWNGLT3 _bp_ship_2) true false)
      (Variables|Default|SetLTB1 false)
      (else
        (Development|SetHiddeninGame (Variables|/Game/SpaceShip/SpaceShip_Final1.SpaceShip_Final1_C|GetWNGLT _bp_ship) false false)
        (Development|SetHiddeninGame (Variables|/Game/SpaceShip/SpaceShip_Final1.SpaceShip_Final1_C|GetWNGLT3 _bp_ship) false false)
        (Variables|Default|SetLTB1 true)))
    (Utilities|Time|SetTimerbyFunctionName 0 "TimerLightWNGR" 0.2)
    (else
      (Development|SetHiddeninGame (Variables|/Game/SpaceShip/SpaceShip_Final1.SpaceShip_Final1_C|GetWNGLT _bp_ship_3) true false)
      (Development|SetHiddeninGame (Variables|/Game/SpaceShip/SpaceShip_Final1.SpaceShip_Final1_C|GetWNGLT3 _bp_ship_3) true false)
      (Development|SetHiddeninGame (Variables|/Game/SpaceShip/SpaceShip_Final1.SpaceShip_Final1_C|GetWNGLT2 _bp_ship_3) true false)
      (Development|SetHiddeninGame (Variables|/Game/SpaceShip/SpaceShip_Final1.SpaceShip_Final1_C|GetWNGLT4 _bp_ship_3) true false))))
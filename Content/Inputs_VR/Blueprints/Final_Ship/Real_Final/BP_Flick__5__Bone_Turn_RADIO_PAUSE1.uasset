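; VR cockpit radio pause button for the spaceship, which toggles the radio audio's paused state when the ZeroGPlayer overlaps it.
; BeginPlay positions it at a cockpit socket; Tick re-attaches it to that bone and reapplies radio volume through a sound mix.
; The overlap animates the button in and out.
; It also holds PlayNextSound, uncalled here, which steps through Korean or Chinese tracks according to the radio channel actor.
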(event OnComponentBeginOverlap(Box)
  (params (OverlappedComponent :type Primitive%20Component%20Object%20Reference) (OtherActor :type Actor%20Object%20Reference) (OtherComp :type Primitive%20Component%20Object%20Reference) (OtherBodyIndex :type Integer) (bFromSweep :type Boolean) (SweepResult :type Hit%20Result%20Structure%20%28by%20ref%29))
  (Utilities|Casting|CastToZeroGPlayer OtherActor)
  (Components|MoveComponentTo (Variables|Default|GetButton) (- (Variables|Default|GetButtonStart) "0.000000,-0.500000,0.000000") "0, 0, 0" false false 0.1 false)
  (bind _output_get (Variables|Default|SetPause (not (Variables|Default|GetPause))))
  (Class|AudioComponent|SetPaused (Variables|Default|GetAudio) _output_get))

(event OnComponentEndOverlap(Box)
  (params (OverlappedComponent :type Primitive%20Component%20Object%20Reference) (OtherActor :type Actor%20Object%20Reference) (OtherComp :type Primitive%20Component%20Object%20Reference) (OtherBodyIndex :type Integer))
  (Utilities|Casting|CastToZeroGPlayer OtherActor)
  (Components|MoveComponentTo (Variables|Default|GetButton) (Variables|Default|GetButtonStart) "0, 0, 0" false false 0.1 false))

(event Custom|PlayNextSound
  (bind _radiochannel (Variables|Default|GetRadioChannel))
  ;[1 1 1] PlaySongs
  (Utilities|FlowControl|Sequence
    (:then_0
      (if (Variables|/Game/Inputs_VR/Blueprints/Final_Ship/Real_Final/Flick__5__Bone_Turn_RADIO_CHANNEL.Flick__5__Bone_Turn_RADIO_CHANNEL_C|GetKorean%20radio _radiochannel)
        (bind _output_get (Variables|Default|SetCurrentSound (Utilities|Array|Get(acopy) (Variables|Default|GetKoreanArray) (Variables|Default|GetCurrentSoundIndexKorean))))
        (Audio|Components|Audio|SetSound (Variables|Default|GetAudio) _output_get)
        (Audio|Components|Audio|Play (Variables|Default|GetAudio) 0.0)
        (Utilities|FlowControl|Delay (Variables|/Script/Engine.SoundBase|GetDuration _output_get))
        (Variables|Default|SetCurrentSoundIndexKorean (+ (Variables|Default|GetCurrentSoundIndexKorean) 1))
        (if (> (Variables|Default|GetCurrentSoundIndexKorean) 1)
          (Variables|Default|SetCurrentSoundIndexChinese 0)
          (if (< (Variables|Default|GetCurrentSoundIndexKorean) (Utilities|Array|Length (Variables|Default|GetKoreanArray)))
            (CallFunction|PlayNextSound)))))
    (:then_1
      (if (Variables|/Game/Inputs_VR/Blueprints/Final_Ship/Real_Final/Flick__5__Bone_Turn_RADIO_CHANNEL.Flick__5__Bone_Turn_RADIO_CHANNEL_C|GetChinese%20radio _radiochannel)
        (bind _output_get_2 (Variables|Default|SetCurrentSound (Utilities|Array|Get(acopy) (Variables|Default|GetChineseArray) (Variables|Default|GetCurrentSoundIndexChinese))))
        (Audio|Components|Audio|SetSound (Variables|Default|GetAudio) _output_get_2)
        (Audio|Components|Audio|Play (Variables|Default|GetAudio) 0.0)
        (Utilities|FlowControl|Delay (Variables|/Script/Engine.SoundBase|GetDuration _output_get_2))
        (Variables|Default|SetCurrentSoundIndexChinese (+ (Variables|Default|GetCurrentSoundIndexChinese) 1))
        (if (> (Variables|Default|GetCurrentSoundIndexChinese) 2)
          (Variables|Default|SetCurrentSoundIndexChinese 0)
          (if (< (Variables|Default|GetCurrentSoundIndexChinese) (Utilities|Array|Length (Variables|Default|GetChineseArray)))
            (CallFunction|PlayNextSound)))))))

(event EventBeginPlay
  (bind _flick__5__bone_turn_radio_pause (Variables|Default|GetFlick__5__Bone_Turn_RADIO_PAUSE))
  (Utilities|FlowControl|Sequence
    (:then_0
      (Variables|Default|SetButtonStart (Variables|/Script/Engine.SceneComponent|GetRelativeLocation (Variables|Default|GetButton))))
    (:then_1
      (bind _returnvalue (Actor|GetActorOfClass "/Game/Zero_Gravity/Blueprints/ZeroGPlayer.ZeroGPlayer_C"))
      (Variables|Default|SetActor _returnvalue)
      (bind _returnvalue_2 (Actor|GetActorOfClass "/Game/SpaceShip/SpaceShip_Final1.SpaceShip_Final1_C"))
      (Variables|Default|SetBP_Ship _returnvalue_2)
      (bind _returnvalue_3 (Actor|GetActorOfClass "/Game/Inputs_VR/Blueprints/Final_Ship/Real_Final/Flick__5__Bone_Turn_RADIO_CHANNEL.Flick__5__Bone_Turn_RADIO_CHANNEL_C"))
      (Variables|Default|SetRadioChannel _returnvalue_3)
      (Transformation|SetWorldTransform _flick__5__bone_turn_radio_pause (Math|Transform|MakeTransform (Transformation|GetSocketLocation (Variables|/Game/SpaceShip/SpaceShip_Final1.SpaceShip_Final1_C|GetCockpit (Variables|Default|GetBP_Ship)) (Utilities|String|StringToName (Utilities|String|Replace (Utilities|GetObjectName _flick__5__bone_turn_radio_pause) (Utilities|String|ToString(Text) (Variables|Default|GetBlender_Name))))) (Math|Rotator|MakeRotator (Variables|Default|GetX%20%28Roll%29) (Variables|Default|GetY%20%28Pitch%29) (Variables|Default|GetZ%20%28Yaw%29)) "1.000000,1.000000,1.000000") false true))
    (:then_2
      ;[1 1 1] PlaySongs
      (Variables|Default|SetChineseArray (Utilities|Array|MakeArray (Variables|Default|Getchinese1) (Variables|Default|Getchinese2) (Variables|Default|GetChinese3)))
      (Variables|Default|SetKoreanArray (Utilities|Array|MakeArray (Variables|Default|Getkorean1) (Variables|Default|Getkorean2))))))

(event EventTick
  (params (DeltaSeconds :type Float%20%28single-precision%29))
  (Utilities|FlowControl|Sequence
    (:then_0
      (if (Utilities|Operators|EqualEqual :A (Variables|/Script/Engine.SceneComponent|GetRelativeLocation (Variables|Default|GetButton)))
        _))
    (:then_1
      (Transformation|AttachComponentToComponent (Variables|/Game/SpaceShip/SpaceShip_Final1.SpaceShip_Final1_C|GetCockpit (Variables|Default|GetBP_Ship)) "Bone_Turn_RADIO_PAUSE" "KeepWorld" "KeepWorld" "KeepWorld" true))
    (:then_2
      (Audio|SetSoundMixClassOverride "/Game/Sound/MasterSoundMixClass.MasterSoundMixClass" "/Engine/EngineSounds/Master.Master" (Variables|Default|GetRadioVolume) 1.0 0.0 true)
      (Audio|PushSoundMixModifier "/Game/Sound/MasterSoundMixClass.MasterSoundMixClass"))))

(fn ConstructionScript)
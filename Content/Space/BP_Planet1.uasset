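; BP_Planet1 is a planet actor that sizes its sphere mesh and gravity field radius from RadiusKm.
; When flagged as ClosestPlanet, it hides the sphere in game and moves a referenced VoxelWorld, scaled to the radius, and a SunSky to its location.
; The SunSky's atmosphere bottom radius and height are set to fit the planet.
; UpdatePlanet does this work, and the construction script calls it, then repeats the ClosestPlanet steps.
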(event EventBeginPlay)

(event Collision|EventActorBeginOverlap
  (params (OtherActor :type Actor%20Object%20Reference)))

(event EventTick
  (params (DeltaSeconds :type Float%20%28single-precision%29)))

(fn ConstructionScript
  (bind _voxelworld (Variables|Default|GetVoxelWorld))
  (bind _sunsky (Variables|Default|GetSunSKy))
  (bind _skyatmospherecomponent (Variables|/Script/Engine.SkyAtmosphere|GetSkyAtmosphereComponent _sunsky))
  (CallFunction|UpdatePlanet)
  (Development|SetHiddeninGame (Variables|Default|GetPlanetSphere) (Variables|Default|GetClosestPlanet) false)
  (if (Variables|Default|GetClosestPlanet)
    (Utilities|FlowControl|Sequence
      (:then_0
        (Variables|Default|GetVoxelWorld
          (:then
            (Transformation|SetActorScale3D _voxelworld (Math|Conversions|ToVector(Float) (Variables|Default|GetRadius%28Km%29)))
            (Transformation|SetActorLocation _voxelworld (Transformation|GetActorLocation) false false))
          (:else)))
      (:then_1
        (Class|SkyAtmosphereComponent|SetBottomRadius _skyatmospherecomponent (- (Variables|Default|GetRadius%28Km%29) 1.0))
        (Transformation|SetActorLocation _sunsky (Transformation|GetActorLocation) false false)
        (Class|SkyAtmosphereComponent|SetAtmosphereHeight _skyatmospherecomponent (Variables|Default|GetAtmosphere%20height))))))

(fn UpdatePlanet
  (bind _voxelworld (Variables|Default|GetVoxelWorld))
  (bind _sunsky (Variables|Default|GetSunSKy))
  (bind _skyatmospherecomponent (Variables|/Script/Engine.SkyAtmosphere|GetSkyAtmosphereComponent _sunsky))
  (Transformation|SetWorldScale3D (Variables|Default|GetPlanetSphere) (Math|Conversions|ToVector(Float) (* (Variables|Default|GetRadius%28Km%29) 2.0 1e+03)))
  (Variables|Default|SetGravityFieldRadius (* (Variables|Default|GetRadius%28Km%29) 1.2 1e+05))
  (Development|SetHiddeninGame (Variables|Default|GetPlanetSphere) (Variables|Default|GetClosestPlanet) false)
  (if (Variables|Default|GetClosestPlanet)
    (Utilities|FlowControl|Sequence
      (:then_0
        (Variables|Default|GetVoxelWorld
          (:then
            (Transformation|SetActorScale3D _voxelworld (Math|Conversions|ToVector(Float) (Variables|Default|GetRadius%28Km%29)))
            (Transformation|SetActorLocation _voxelworld (Transformation|GetActorLocation) false false))
          (:else)))
      (:then_1
        (Class|SkyAtmosphereComponent|SetBottomRadius _skyatmospherecomponent (- (Variables|Default|GetRadius%28Km%29) 1.0))
        (Transformation|SetActorLocation _sunsky (Transformation|GetActorLocation) false false)
        (Class|SkyAtmosphereComponent|SetAtmosphereHeight _skyatmospherecomponent (Variables|Default|GetAtmosphere%20height))))))
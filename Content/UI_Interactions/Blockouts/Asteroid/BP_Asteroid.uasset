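; Mineable asteroid that, once destroyed, breaks apart and is sucked into the player's gun sphere as ore.
; GetDestroyed uses a delayed loop to release each static mesh in turn, disabling collision and recording its scale and distance.
; Tick pulls released pieces with capped, time-based acceleration, shrinking them by remaining distance.
; Each piece reaching the sphere is removed and adds random amounts of the flagged ore types to the ZeroGPlayer.
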(event Custom|Pull
  (params (Bit :type Asteroid%20Info%20Structure))
  (bind (_staticmeshcomp _maxdist _defaultscl) (Utilities|Struct|BreakAsteroidInfo Bit))
  (bind _player (Variables|Default|GetPlayer))
  (bind _player_2 (Variables|Default|GetPlayer))
  (bind _gunsuckywucky (Variables|Default|GetGunSuckyWucky))
  (bind _player_3 (Variables|Default|GetPlayer))
  (bind _player_4 (Variables|Default|GetPlayer))
  (bind _player_5 (Variables|Default|GetPlayer))
  (bind _returnvalue (Transformation|GetWorldLocation _staticmeshcomp))
  (bind _returnvalue_2 (Transformation|GetWorldLocation _gunsuckywucky))
  (bind _returnvalue_3 (Math|Vector|Distance(Vector) _returnvalue _returnvalue_2))
  (bind _returnvalue_4 (/ _returnvalue_3 _maxdist))
  (bind _returnvalue_5 (* _defaultscl _returnvalue_4))
  (bind _returnvalue_6 (+ _returnvalue_5 0.01))
  (Utilities|IsValid _staticmeshcomp
    (:Is%20Valid
      (Transformation|AddLocalOffset _staticmeshcomp (* (Math|Vector|Normalize (- _returnvalue_2 _returnvalue)) (Utilities|Time|GetWorldDeltaSeconds) (Math|Float|Min(Float) (+ (Math|Float|Power (Variables|Default|GetSpeed) (Variables|Default|GetTimeSince)) 1.5e+02) 2.6e+02)) false false)
      (Transformation|SetWorldScale3D _staticmeshcomp (Math|Vector|MakeVector _returnvalue_6 _returnvalue_6 _returnvalue_6))
      (if (<= _returnvalue_3 1e+01)
        (Components|DestroyComponent _staticmeshcomp)
        (Utilities|FlowControl|Sequence
          (:then_0
            (if (Variables|Default|GetZinc)
              (Variables|/Game/Zero_Gravity/Blueprints/ZeroGPlayer.ZeroGPlayer_C|SetZincOre _player_4 (+ (Variables|/Game/Zero_Gravity/Blueprints/ZeroGPlayer.ZeroGPlayer_C|GetZincOre (Variables|Default|GetPlayer)) (Math|Random|RandomFloatinRange 0.0 15.0)))
              (Development|PrintString (Utilities|String|Append (Utilities|String|ToString(Float) (Variables|/Game/Zero_Gravity/Blueprints/ZeroGPlayer.ZeroGPlayer_C|GetZincOre _player_4)) "Iron"))))
          (:then_1
            (if (Variables|Default|GetCopper)
              (Variables|/Game/Zero_Gravity/Blueprints/ZeroGPlayer.ZeroGPlayer_C|SetCopperOre _player (+ (Variables|/Game/Zero_Gravity/Blueprints/ZeroGPlayer.ZeroGPlayer_C|GetCopperOre (Variables|Default|GetPlayer)) (Math|Random|RandomFloatinRange 0.0 2e+01)))
              (Development|PrintString (Utilities|String|Append (Utilities|String|ToString(Float) (Variables|/Game/Zero_Gravity/Blueprints/ZeroGPlayer.ZeroGPlayer_C|GetCopperOre _player)) "Gold"))))
          (:then_2
            (if (Variables|Default|GetAcidic%20Crystal)
              (Variables|/Game/Zero_Gravity/Blueprints/ZeroGPlayer.ZeroGPlayer_C|SetAcidicCrystal _player_2 (+ (Variables|/Game/Zero_Gravity/Blueprints/ZeroGPlayer.ZeroGPlayer_C|GetAcidicCrystal (Variables|Default|GetPlayer)) (Math|Random|RandomFloatinRange 0.0 5.0)))
              (Development|PrintString (Utilities|String|Append (Utilities|String|ToString(Float) (Variables|/Game/Zero_Gravity/Blueprints/ZeroGPlayer.ZeroGPlayer_C|GetAcidicCrystal _player_2)) "Rock"))))
          (:then_3
            (if (Variables|Default|GetPolymer)
              (Variables|/Game/Zero_Gravity/Blueprints/ZeroGPlayer.ZeroGPlayer_C|SetPolymer _player_3 (+ (Variables|/Game/Zero_Gravity/Blueprints/ZeroGPlayer.ZeroGPlayer_C|GetPolymer (Variables|Default|GetPlayer)) (Math|Random|RandomFloatinRange 0.0 3.0)))
              (Development|PrintString (Utilities|String|Append (Utilities|String|ToString(Float) (Variables|/Game/Zero_Gravity/Blueprints/ZeroGPlayer.ZeroGPlayer_C|GetPolymer _player_3)) "Rock"))))
          (:then_4
            (if (Variables|Default|GetTitanium)
              (Variables|/Game/Zero_Gravity/Blueprints/ZeroGPlayer.ZeroGPlayer_C|SetTitaniumOre _player_5 (+ (Variables|/Game/Zero_Gravity/Blueprints/ZeroGPlayer.ZeroGPlayer_C|GetTitaniumOre (Variables|Default|GetPlayer)) (Math|Random|RandomFloatinRange 0.0 5.0)))
              (Development|PrintString (Utilities|String|Append (Utilities|String|ToString(Float) (Variables|/Game/Zero_Gravity/Blueprints/ZeroGPlayer.ZeroGPlayer_C|GetTitaniumOre _player_5)) "Rock")))))))))

(event Custom|GetDestroyed
  (bind _returnvalue (Math|Random|RandomFloatinRange -1.0 1.0))
  ;[1 1 1] If ball hits Asteroid
  (Variables|Default|SetIsDestroyed true)
  (bind _array_element (Utilities|ForEachwithDelay (Variables|Default|GetAllRocks) 0.05)
    (:Loop%20Body
      (Collision|SetCollisionEnabled _array_element "NoCollision")
      (Utilities|Array|Add (Variables|Default|GetAllBits) (Utilities|Struct|MakeAsteroidInfo _array_element (Math|Vector|Distance(Vector) (Transformation|GetWorldLocation (Variables|Default|GetGunSuckyWucky)) (Transformation|GetWorldLocation _array_element)) (.x (Transformation|GetWorldScale _array_element)) true))
      (Transformation|AddLocalRotation _array_element (Math|Rotator|MakeRotator _returnvalue _returnvalue _returnvalue) false false))))

(event EventBeginPlay
  (bind _returnvalue (Actor|GetActorOfClass "/Game/Zero_Gravity/Blueprints/ZeroGPlayer.ZeroGPlayer_C"))
  (Variables|Default|SetPlayer _returnvalue)
  (Variables|Default|SetAllRocks (Actor|GetComponentsByClass "/Script/Engine.StaticMeshComponent"))
  (bind _aszero_gplayer (Utilities|Casting|CastToZeroGPlayer (Pawn|GetControlledPawn (Game|GetPlayerController 0))))
  (Variables|Default|SetGunSuckyWucky (Variables|/Game/Zero_Gravity/Blueprints/ZeroGPlayer.ZeroGPlayer_C|GetSphere _aszero_gplayer)))

(event EventTick
  (params (DeltaSeconds :type Float%20%28single-precision%29))
  (if (Variables|Default|GetIsDestroyed)
    (Variables|Default|SetTimeSince (+ (Variables|Default|GetTimeSince) DeltaSeconds))
    (for _array_element (Variables|Default|GetAllBits)
      (if (.IsDestroyed (Utilities|Struct|BreakAsteroidInfo _array_element))
        (CallFunction|Pull _array_element)))))

(fn ConstructionScript)
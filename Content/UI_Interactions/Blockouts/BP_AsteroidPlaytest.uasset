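; Playtest asteroid that breaks apart when destroyed and gets sucked into the UIZeroGPlayer pawn's Sphere component.
; GetDestroyed staggers through the actor's static mesh components, disabling collision, slightly rotating each and recording its starting distance and scale.
; Tick pulls each recorded bit toward the sphere at an exponentially rising, capped speed.
; Bits shrink in proportion to remaining distance and are destroyed on arrival.
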(event Custom|Pull
  (params (Bit :type Asteroid%20Info%20Structure))
  (bind (_staticmeshcomp _maxdist _defaultscl) (Utilities|Struct|BreakAsteroidInfo Bit))
  (bind _gunsuckywucky (Variables|Default|GetGunSuckyWucky))
  (bind _returnvalue (Transformation|GetWorldLocation _staticmeshcomp))
  (bind _returnvalue_2 (Transformation|GetWorldLocation _gunsuckywucky))
  (bind _returnvalue_3 (Math|Vector|Distance(Vector) _returnvalue _returnvalue_2))
  (bind _returnvalue_4 (/ _returnvalue_3 _maxdist))
  (bind _returnvalue_5 (* _defaultscl _returnvalue_4))
  (bind _returnvalue_6 (+ _returnvalue_5 0.01))
  (Utilities|IsValid _staticmeshcomp
    (:Is%20Valid
      (Transformation|AddLocalOffset _staticmeshcomp (* (Math|Vector|Normalize (- _returnvalue_2 _returnvalue)) (Utilities|Time|GetWorldDeltaSeconds) (Math|Float|Min(Float) (+ (Math|Float|Power (Variables|Default|GetSpeed) (Variables|Default|GetTimeSince)) 1.5e+02) 2.6e+02)) false false)
      (Transformation|SetWorldScale3D _staticmeshcomp (Math|Vector|MakeVector _returnvalue_6 _returnvalue_6 _returnvalue_6))
      (if (<= _returnvalue_3 1e+01)
        (Components|DestroyComponent _staticmeshcomp)))))

(event Custom|GetDestroyed
  (bind _returnvalue (Math|Random|RandomFloatinRange -1.0 1.0))
  ;[1 1 1] If ball hits Asteroid
  (Variables|Default|SetIsDestroyed true)
  (bind _array_element (Utilities|ForEachwithDelay (Variables|Default|GetAllRocks) 0.05)
    (:Loop%20Body
      (Collision|SetCollisionEnabled _array_element "NoCollision")
      (Utilities|Array|Add (Variables|Default|GetAllBits) (Utilities|Struct|MakeAsteroidInfo _array_element (Math|Vector|Distance(Vector) (Transformation|GetWorldLocation (Variables|Default|GetGunSuckyWucky)) (Transformation|GetWorldLocation _array_element)) (.x (Transformation|GetWorldScale _array_element)) true))
      (Transformation|AddLocalRotation _array_element (Math|Rotator|MakeRotator _returnvalue _returnvalue _returnvalue) false false))))

(event EventBeginPlay
  (Variables|Default|SetAllRocks (Actor|GetComponentsByClass "/Script/Engine.StaticMeshComponent"))
  (bind _asuizero_gplayer (Utilities|Casting|CastToUIZeroGPlayer (Pawn|GetControlledPawn (Game|GetPlayerController 0))))
  (Variables|Default|SetGunSuckyWucky (Variables|/Game/UI_Interactions/UIZeroGPlayer.UIZeroGPlayer_C|GetSphere _asuizero_gplayer)))

(event Collision|EventActorBeginOverlap
  (params (OtherActor :type Actor%20Object%20Reference)))

(event EventTick
  (params (DeltaSeconds :type Float%20%28single-precision%29))
  (if (Variables|Default|GetIsDestroyed)
    (Variables|Default|SetTimeSince (+ (Variables|Default|GetTimeSince) DeltaSeconds))
    (for _array_element (Variables|Default|GetAllBits)
      (if (.IsDestroyed (Utilities|Struct|BreakAsteroidInfo _array_element))
        (CallFunction|Pull _array_element)))))

(fn ConstructionScript)
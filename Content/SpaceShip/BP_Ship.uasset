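; Pilotable spaceship that seats the player on cockpit overlap using timers to glide them in, attach them to the chair and play the cockpit animation.
; Tick sets physics velocity from thruster speed plus a gravity term and applies joystick torque, with roll from input; hyper-thrust interpolation is immediately overwritten by thruster speed.
; Enter and Exit swap possession, and the construction script snaps name-matched meshes to cockpit sockets.
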(event OnComponentBeginOverlap(CockPitColl)
  (params (OverlappedComponent :type Primitive%20Component%20Object%20Reference) (OtherActor :type Actor%20Object%20Reference) (OtherComp :type Primitive%20Component%20Object%20Reference) (OtherBodyIndex :type Integer) (bFromSweep :type Boolean) (SweepResult :type Hit%20Result%20Structure%20%28by%20ref%29))
  ;[1 1 1] Set pawn in cockpit chair
  (if (== OtherActor (Game|Player|GetPlayerPawn 0))
    (Development|PrintString "PlayerOverlapping")
    (Utilities|FlowControl|DoOnce false
      (:Completed
        (bind _returnvalue (Utilities|Time|SetTimerbyFunctionName 0 "SetRotationCockpit" 0.01 true 0.0 0.1))
        (Variables|Default|SetRotationCockpit _returnvalue)
        (Utilities|Time|SetTimerbyFunctionName 0 "PlayCockpitAnimation" 0.01 false 5.0)
        (Utilities|Time|SetTimerbyFunctionName 0 "SyncPositionCockpit" 0.01 true 3.0)
        (Collision|SetCollisionEnabled (Variables|Default|GetCockPitColl) "NoCollision")))))

(event Input|EnhancedActionEvents|EnhancedInputActionIA_ShipFB
  (params (ActionValue :type Vector%202D%20Structure) (ElapsedSeconds :type Float%20%28double-precision%29) (TriggeredSeconds :type Float%20%28double-precision%29) (InputAction :type Input%20Action%20Object%20Reference :default "/Game/VRTemplate/Input/Actions/SpaceShip/IA_ShipFB.IA_ShipFB"))
  ;[1 1 1] Ship rotation based on joystick input
  (Class|PrimitiveComponent|AddTorqueinDegrees (Variables|Default|GetShip) (* (Math|Vector|GetRightVector (Variables|Default|GetShip)) (* (Variables|/Game/Inputs_VR/Blueprints/Joystick.Joystick_C|GetVariable%20max%20y (Variables|Default|GetJoystick)) (Variables|Default|GetForwardTorquePower))) "None" true))

(event Input|EnhancedActionEvents|EnhancedInputActionIA_ShipMoveRight
  (params (ActionValue :type Vector%202D%20Structure) (ElapsedSeconds :type Float%20%28double-precision%29) (TriggeredSeconds :type Float%20%28double-precision%29) (InputAction :type Input%20Action%20Object%20Reference :default "/Game/VRTemplate/Input/Actions/SpaceShip/IA_ShipMoveRight.IA_ShipMoveRight"))
  ;[1 1 1] Ship rotation based on joystick input
  (Class|PrimitiveComponent|AddTorqueinDegrees (Variables|Default|GetShip) (* (Math|Vector|GetUpVector (Variables|Default|GetShip)) (* (Variables|/Game/Inputs_VR/Blueprints/Joystick.Joystick_C|Getvariable%20max%20x (Variables|Default|GetJoystick)) (Variables|Default|GetForwardTorquePower))) "None" true))

(event Input|EnhancedActionEvents|EnhancedInputActionEnterExitShip
  (params (ActionValue :type Boolean) (ElapsedSeconds :type Float%20%28double-precision%29) (TriggeredSeconds :type Float%20%28double-precision%29) (InputAction :type Input%20Action%20Object%20Reference :default "/Game/VRTemplate/Input/Actions/SpaceShip/EnterExitShip.EnterExitShip"))
  ;[1 1 1] Ship rotation based on joystick input
  (CallFunction|Exit))

(event Input|EnhancedActionEvents|EnhancedInputActionIA_ShipRoll
  (params (ActionValue :type Vector%202D%20Structure) (ElapsedSeconds :type Float%20%28double-precision%29) (TriggeredSeconds :type Float%20%28double-precision%29) (InputAction :type Input%20Action%20Object%20Reference :default "/Game/VRTemplate/Input/Actions/SpaceShip/IA_ShipRoll.IA_ShipRoll"))
  ;[1 1 1] Ship rotation based on joystick input
  (Class|PrimitiveComponent|AddTorqueinDegrees (Variables|Default|GetShip) (* (Math|Vector|GetForwardVector (Variables|Default|GetShip)) (* ActionValue (Variables|Default|GetForwardTorquePower))) "None" true))

(event Input|EnhancedActionEvents|EnhancedInputActionHyperThrust
  (params (ActionValue :type Float%20%28double-precision%29) (ElapsedSeconds :type Float%20%28double-precision%29) (TriggeredSeconds :type Float%20%28double-precision%29) (InputAction :type Input%20Action%20Object%20Reference :default "/Game/VRTemplate/Input/Actions/SpaceShip/HyperThrust.HyperThrust"))
  ;[1 1 1] Ship thrust
  (:Triggered
    (bind _output_get (Variables|Default|SetSuperSpeed true)))
  (:Completed
    (Variables|Default|SetSuperSpeed false)))

(event EventBeginPlay
  ;[1 1 1] Ship thrust
  (bind _returnvalue (Actor|GetActorOfClass "BP_Ship_C"))
  (Variables|Default|SetBP_Ship _returnvalue)
  (bind _returnvalue_2 (Actor|GetActorOfClass "/Game/Zero_Gravity/Blueprints/ZeroGPlayer.ZeroGPlayer_C"))
  (Variables|Default|SetOccupant _returnvalue_2)
  (bind _returnvalue_3 (Actor|GetActorOfClass "/Game/Inputs_VR/Blueprints/Joystick.Joystick_C"))
  (Variables|Default|SetJoystick _returnvalue_3)
  (bind _returnvalue_4 (Actor|GetActorOfClass "/Game/Inputs_VR/Blueprints/Landing_Gear.Landing_Gear_C"))
  (Variables|Default|SetLanding_gear _returnvalue_4)
  (bind _returnvalue_5 (Actor|GetActorOfClass "/Game/Inputs_VR/Blueprints/Thruster_Ship.Thruster_Ship_C"))
  (Variables|Default|SetThrusters _returnvalue_5))

(event EventTick
  (params (DeltaSeconds :type Float%20%28single-precision%29))
  (bind _test (Variables|Default|Gettest))
  ;[1 1 1] Set velocity forward
  (Utilities|FlowControl|Sequence
    (:then_0
      (if (< (Math|Vector|VectorLength (Variables|Default|GetForwardVelocity)) (Variables|Default|GetGravityThreshold))
        (Variables|Default|SetUpwardsVelocity (* (Math|Float|Lerp 0.0 -9.8e+02 (- (Math|Vector|VectorLength (Variables|Default|GetForwardVelocity)) (Variables|Default|GetGravityThreshold))) (Math|Vector|UnrotateVector (Math|Vector|GetUpVector (Variables|Default|GetShip)) (Transformation|GetWorldRotation (Variables|Default|GetShip)))))
        (else
          (Variables|Default|SetUpwardsVelocity (Math|Interpolation|VInterpTo (Variables|Default|GetUpwardsVelocity) "0, 0, 0" (Utilities|Time|GetWorldDeltaSeconds) 0.0)))))
    (:then_1
      (Physics|SetPhysicsLinearVelocity (Variables|Default|GetShip) (* (+ (Variables|Default|GetForwardVelocity) (Variables|Default|GetUpwardsVelocity)) "-1.000000,-1.000000,-1.000000") false "None"))
    (:then_2
      ;[1 1 1] Ship rotation based on joystick input
      (Class|PrimitiveComponent|AddTorqueinDegrees (Variables|Default|GetShip) (* (Math|Vector|GetRightVector (Variables|Default|GetShip)) (* (Variables|/Game/Inputs_VR/Blueprints/Joystick.Joystick_C|GetVariable%20max%20y (Variables|Default|GetJoystick)) (Variables|Default|GetForwardTorquePower))) "None" true))
    (:then_3
      (Class|PrimitiveComponent|AddTorqueinDegrees (Variables|Default|GetShip) (* (Math|Vector|GetUpVector (Variables|Default|GetShip)) (* (Variables|/Game/Inputs_VR/Blueprints/Joystick.Joystick_C|Getvariable%20max%20x (Variables|Default|GetJoystick)) (Variables|Default|GetForwardTorquePower))) "None" true))
    (:then_4
      ;[1 1 1] Ship thrust
      (Utilities|FlowControl|Sequence
        (:then_0
          (if (stale Input|EnhancedActionEvents|EnhancedInputActionHyperThrust _output_get)
            (if (not (Math|Float|NearlyEqual(Float) _test 0.0 0.1))
              (Variables|Default|SetThrust (Math|Interpolation|FInterpTo (Variables|Default|GetThrust) (Math|Float|Lerp 0.0 (Variables|Default|GetMaxThrust) (/ (+ _test 1.0) 0.1)) (Utilities|Time|GetWorldDeltaSeconds) 0.5)))
            (elif (not (Math|Float|NearlyEqual(Float) _test 0.0 0.1))
              (bind _output_get (Variables|Default|SetThrust (Math|Interpolation|FInterpTo (Variables|Default|GetThrust) (Math|Float|Lerp 0.0 (Variables|Default|GetMaxThrust) (/ (+ _test 0.0) 2.0)) (Utilities|Time|GetWorldDeltaSeconds) 0.5)))
              (Development|PrintString (Utilities|String|ToString(Float) _output_get)))))
        (:then_1
          (bind _output_get_2 (Variables|Default|SetThrust (Variables|/Game/Inputs_VR/Blueprints/Thruster_Ship.Thruster_Ship_C|GetThrusterSpeed (Variables|Default|GetThrusters))))
          (Variables|Default|SetForwardVelocity (* (* (* (Math|Vector|GetForwardVector (Variables|Default|GetShip)) (Variables|Default|GetThrust)) "-1.000000,-1.000000,-1.000000") "7.000000,7.000000,7.000000")))))))

(event Input|ActionEvents|InputActionSuperSonics
  (params (Key :type Key%20Structure :default "None"))
  ;[1 1 1] Ship thrust
)

(event Input|AxisEvents|InputAxisIA_SHIPFB
  (params (AxisValue :type Float%20%28single-precision%29))
  ;[1 1 1] Ship rotation based on joystick input
)

(event Input|AxisEvents|InputAxisMoveRight
  (params (AxisValue :type Float%20%28single-precision%29))
  ;[1 1 1] Ship rotation based on joystick input
)

(event Input|AxisEvents|InputAxisRoll
  (params (AxisValue :type Float%20%28single-precision%29))
  ;[1 1 1] Ship rotation based on joystick input
)

(fn ConstructionScript
  (bind _cockpit (Variables|Default|GetCockpit))
  (for _array_element (Actor|GetComponentsByClass "/Script/Engine.StaticMeshComponent")
    (if (Utilities|String|Contains (Utilities|GetDisplayName _array_element) (Utilities|String|ToString(Text) (Variables|Default|GetBlender_Name)))
      (Transformation|SetWorldTransform _array_element (Math|Transform|MakeTransform (Transformation|GetSocketLocation _cockpit (Utilities|String|StringToName (Utilities|String|Replace (Utilities|GetObjectName _array_element) (Utilities|String|ToString(Text) (Variables|Default|GetBlender_Name))))) (Math|Rotator|MakeRotator (.roll (Transformation|GetSocketRotation _cockpit (Utilities|String|StringToName (Utilities|String|Replace (Utilities|GetObjectName _array_element) (Utilities|String|ToString(Text) (Variables|Default|GetBlender_Name)))))) (.pitch (Transformation|GetSocketRotation _cockpit (Utilities|String|StringToName (Utilities|String|Replace (Utilities|GetObjectName _array_element) (Utilities|String|ToString(Text) (Variables|Default|GetBlender_Name)))))) (.yaw (Transformation|GetSocketRotation _cockpit (Utilities|String|StringToName (Utilities|String|Replace (Utilities|GetObjectName _array_element) (Utilities|String|ToString(Text) (Variables|Default|GetBlender_Name))))))) (Transformation|GetWorldScale _array_element)) false true)
      (Transformation|AttachComponentToComponent _array_element (Variables|Default|GetCockpit) (Utilities|String|StringToName (Utilities|String|Replace (Utilities|GetObjectName _array_element) (Utilities|String|ToString(Text) (Variables|Default|GetBlender_Name)))) "SnapToTarget" "SnapToTarget" "KeepWorld" true))))

(fn Enter
  (params (ExitDelegate :type Delegate%20%28by%20ref%29) (Player :type Zero%20G%20Player%20Object%20Reference))
  (EventDispatchers|BindEventtoOnExited ExitDelegate)
  (bind _output_get (Variables|Default|SetOccupant Player))
  (Pawn|Possess (Pawn|GetController _output_get) self)
  (Transformation|AttachActorToActor (Variables|Default|GetOccupant) self "Pilot" "SnapToTarget" "SnapToTarget" "SnapToTarget" true))

(fn SyncPositionCockpit
  (Utilities|Time|ClearandInvalidateTimerbyHandle (Variables|Default|GetRotationCockpit))
  (Transformation|AttachComponentToComponent (Variables|Default|GetOccupant) (Variables|BP_Ship_C|GetCockpit (Variables|Default|GetBP_Ship)) "Chair" "SnapToTarget" "SnapToTarget" "KeepWorld" true))

(fn Exit
  (Transformation|DetachFromActor (Variables|Default|GetOccupant) "KeepWorld" "KeepWorld" "KeepWorld")
  (Transformation|SetActorLocation (Variables|Default|GetOccupant) (Transformation|GetWorldLocation (Variables|Default|GetBox)) false false)
  (Pawn|Possess (Pawn|GetController) (Variables|Default|GetOccupant)))

(fn SetRotationCockpit
  (bind _occupant (Variables|Default|GetOccupant))
  (bind _occupant_2 (Variables|Default|GetOccupant))
  (Variables|Default|SetSetRotationcockpitt true)
  (if true
    (Transformation|SetActorRotation _occupant (Math|Interpolation|RInterpTo (Variables|/Script/Engine.SceneComponent|GetRelativeRotation (Variables|/Script/Engine.Character|GetCapsuleComponent _occupant)) (Variables|/Script/Engine.SceneComponent|GetRelativeRotation (Variables|Default|GetPoint%20to%20move%20too)) (Utilities|Time|GetWorldDeltaSeconds) 0.5))
    (Transformation|SetActorLocation _occupant_2 (Math|Interpolation|VInterpTo (Transformation|GetActorLocation _occupant_2) (Transformation|GetWorldLocation (Variables|Default|GetPoint%20to%20move%20too)) (Utilities|Time|GetWorldDeltaSeconds) 0.5) false false)
    (Variables|Default|SetSetRotationcockpitt false)))

(fn PlayCockpitAnimation
  (Components|Animation|PlayAnimation (Variables|BP_Ship_C|GetCockpit (Variables|Default|GetBP_Ship)) "/Game/SpaceShip/SpaceSHip/Cockpitu/CockPit__1__Anim.CockPit__1__Anim" false))

(fn SyncButtons
  (bind _cockpit (Variables|Default|GetCockpit))
  (for _array_element (Actor|GetComponentsByClass "/Script/Engine.StaticMeshComponent")
    (if (Utilities|String|Contains (Utilities|GetDisplayName _array_element) (Utilities|String|ToString(Text) (Variables|Default|GetBlender_Name)))
      (Transformation|SetWorldTransform _array_element (Math|Transform|MakeTransform (Transformation|GetSocketLocation _cockpit (Utilities|String|StringToName (Utilities|String|Replace (Utilities|GetObjectName _array_element) (Utilities|String|ToString(Text) (Variables|Default|GetBlender_Name))))) (Math|Rotator|MakeRotator (.roll (Transformation|GetSocketRotation _cockpit (Utilities|String|StringToName (Utilities|String|Replace (Utilities|GetObjectName _array_element) (Utilities|String|ToString(Text) (Variables|Default|GetBlender_Name)))))) (.pitch (Transformation|GetSocketRotation _cockpit (Utilities|String|StringToName (Utilities|String|Replace (Utilities|GetObjectName _array_element) (Utilities|String|ToString(Text) (Variables|Default|GetBlender_Name)))))) (.yaw (Transformation|GetSocketRotation _cockpit (Utilities|String|StringToName (Utilities|String|Replace (Utilities|GetObjectName _array_element) (Utilities|String|ToString(Text) (Variables|Default|GetBlender_Name))))))) (Transformation|GetWorldScale _array_element)) false true))))